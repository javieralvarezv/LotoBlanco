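; VisualSound is an expanding sound-wave actor that toggles the visibility of the geometry it hits.
; Each Tick it eases its scale toward the initial scale plus MaxRadius at a rate set by GrowingSpeed, then destroys itself on reaching that size.
; On overlap it calls Touched on the other actor's ObstacleComponent, passing its sound color, first-round flag and whether a character spawned it.
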(event `self.ReceiveBeginPlay`
  ;[0 0 0] Establecemos el tamaño máximo
  (bind _output_get (set `self.Initial Scale` (`self.GetActorScale3D`)))
  (set `self.Maximun Scale` (+ _output_get (`self.Max Radius`))))

(event `self.ReceiveTick`
  (params (DeltaSeconds :type "Float (single-precision)"))
  ;[0 0 0] Interpolamos la escala del actor
  (`self.ActorScaleLerp` DeltaSeconds)
  ;[0 0 0] Si se alcanza la escala máxima se elimina el actor
  (if (== (`self.GetActorScale3D`) (`self.Maximun Scale`) :`ErrorTolerance` 0.01)
    (`self.K2_DestroyActor`)))

(event `self.ReceiveActorBeginOverlap`
  (params (OtherActor :type "Actor Object Reference"))
  ;[0 0 0] Hacemos visible o invisible la geometría con la que choca
  (bind _output_get (set `self.Obstacle Component Reference` (`self.GetComponentByClass` OtherActor "/Game/Blueprints/ObstacleComponent.ObstacleComponent_C")))
  (`/Engine/EditorBlueprintResources/StandardMacros.IsValid` _output_get
    (:`Is Valid`
      (`/Game/Blueprints/ObstacleComponent.Touched` (`self.Obstacle Component Reference`) (`self.sound_color`) (`self.first round`) (`self.spawned by character`)))))

(fn `ActorScaleLerp`
  (params (A :type "Float (double-precision)"))
  (`self.SetActorScale3D` (`KismetMathLibrary.VLerp` (`self.GetActorScale3D`) (`self.Maximun Scale`) (* A (`self.Growing Speed`)))))

(fn `UserConstructionScript`)