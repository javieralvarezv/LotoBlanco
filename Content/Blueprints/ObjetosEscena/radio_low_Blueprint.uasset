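; Radio scene object that plays its audio and periodically emits a visual representation of that sound.
; BeginPlay starts the Radio sound at the actor's location and a looping timer.
; While AbleToSound is set, each timer tick spawns a VisualSound actor sized by SoundRadius, flagged as spawned by a character despite coming from the radio.
; The construction script assigns Outline to the Otuline variable.
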(event `self.ReceiveBeginPlay`
  ;[0 0 0] Start
  (`KismetSystemLibrary.K2_SetTimerDelegate` (delegate `SpawnSound`) 1.2 true)
  (`GameplayStatics.SpawnSoundAtLocation` "/Game/sounds/Radio/Radio.Radio" (`self.K2_GetActorLocation`) (struct) 1.0 1.0 0.0 null null))

(event `SpawnSound`
  ;[0 0 0] Spawn sound
  (if (`self.able to sound`)
    (`|SpawnActorFromClass` "/Game/Blueprints/VisualSound.VisualSound_C" (`self.GetTransform`) "Undefined" "OverrideRootScale" null (`self.sound radius`) (struct :`R` 1.0 :`G` 1.0 :`B` 1.0) true null)))

(fn `UserConstructionScript`
  (set `self.otuline` (`self.Outline`)))